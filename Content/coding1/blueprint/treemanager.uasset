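; Tree manager Blueprint that animates Bptreat actors in the level with random leaf wiggles.
; After a startup delay, it caches all Bptreat actors, then WiggleLeaves multiplies their root child components' scales by random factors, so changes compound, and calls itself again after delays.
; An index-driven staggered reveal follows that recursive call, but HideTrees actually unhides every tree and ShowTreesSlowly is empty.
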(event `self.ReceiveBeginPlay`
  (`KismetSystemLibrary.PrintText` "Tree managerr starting up")
  (`KismetSystemLibrary.Delay` 3.0)
  (bind _outactors (`GameplayStatics.GetAllActorsOfClass` "/Game/coding1/blueprint/bptreat.bptreat_C"))
  (set `self.treearray` _outactors) ; promaate to varaiable takes the data and save it for later
  (`self.Wiggle leaves`))

(event `Wiggle leaves`
  (bind _index (`self.index`))
  (for _array_element (`self.treearray`)
    (for _array_element_2 (`SceneComponent.GetChildrenComponents` (`/Game/coding1/blueprint/bptreat.DefaultSceneRoot` _array_element) false)
      (`SceneComponent.SetRelativeScale3D` _array_element_2 (* (`SceneComponent.RelativeScale3D` _array_element_2) (`KismetMathLibrary.RandomFloatInRange` 0.8 1.2))))
    (`KismetSystemLibrary.Delay` 0.5)
    (`self.Wiggle leaves`)
    (`self.hidetrees`)
    (`self.showtreesslowly`)
    (`KismetSystemLibrary.Delay` 1.0)
    (`self.SetActorHiddenInGame` (`|GetArrayItem` (`self.treearray`) _index) false)
    (bind _result (`/Engine/EditorBlueprintResources/StandardMacros.IncrementInt` _index)
      (:`  `
        (if (not (== _result (`KismetArrayLibrary.Array_Length` (`self.treearray`))))
          (`self.showtreesslowly`))))))

(event `hidetrees`
  (for _array_element (`self.treearray`)
    (`self.SetActorHiddenInGame` _array_element false)))

(event `showtreesslowly`)

(fn `UserConstructionScript`)
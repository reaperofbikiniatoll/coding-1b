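; BP_Spawner is a spawner actor that creates instances of a configurable ThingToSpawn class, with debug text suggesting a key.
; SpawnThing spawns the actor at the SpawnPoint component's world transform, skipping the spawn if it would collide.
; With Autospawn enabled, BeginPlay makes the first call and SpawnThing re-calls itself after a fixed delay, forming a repeating loop.
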(event `self.ReceiveBeginPlay`
  (`KismetSystemLibrary.PrintText` "Spawner Active")
  (if (`self.autospawn`)
    (`self.Spawn Thing`)))

(event `Spawn Thing`
  (`KismetSystemLibrary.PrintText` "spawning the key")
  (`|SpawnActorFromClass` (`self.Thing to Spawn`) (`SceneComponent.K2_GetComponentToWorld` (`self.spawn point`)) "DontSpawnIfColliding" "MultiplyWithRoot" null null)
  (if (`self.autospawn`)
    (`KismetSystemLibrary.Delay` 5.0)
    (`self.Spawn Thing`)))

(fn `UserConstructionScript`)